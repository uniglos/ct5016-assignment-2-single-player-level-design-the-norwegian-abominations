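; BP_KeyDoor is a double door that opens when a player holding the matching key enters its trigger box.
; On overlap it searches the BP_Player Key array for a true entry at KeyValue, with a DoOnce guarding re-entry.
; A match plays a timeline rotating both anchors open, then resets that key slot after a brief delay.
; Without a match it briefly shows the W_KeyDoor widget and re-arms the check.
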(event `OpenDoor`
  (bind (_direction _open) (`Timeline|DoorOpen` :!via `PlayFromStart`)
    (:`Update`
      (`SceneComponent.K2_SetRelativeRotation` (`self.RightAnchor`) (`KismetMathLibrary.RLerp` (`self.Closed`) (`self.OpenRight`) _open) false false)
      (`SceneComponent.K2_SetRelativeRotation` (`self.LeftAnchor`) (`KismetMathLibrary.RLerp` (`self.Closed`) (`self.OpenLeft`) _open) false false))
    (:`Finished`
      (`KismetSystemLibrary.Delay` 0.2)
      (`KismetArrayLibrary.Array_Set` (`/Game/Blueprints/BP_Player.Key` (stale `self.Box.OnComponentBeginOverlap` _asbp_player)) (`self.KeyValue`)))))

(event `self.Box.OnComponentBeginOverlap`
  (params (OverlappedComponent :type "PrimitiveComponent Object Reference") (OtherActor :type "Actor Object Reference") (OtherComp :type "PrimitiveComponent Object Reference") (OtherBodyIndex :type Integer) (bFromSweep :type Boolean) (SweepResult :type "HitResult Structure (by ref)"))
  (bind _asbp_player (cast `/Game/Blueprints/BP_Player` OtherActor))
  (`/Engine/EditorBlueprintResources/StandardMacros.DoOnce` false :!label _label
    (:`Completed`
      (for (_array_element _array_index) (`/Game/Blueprints/BP_Player.Key` _asbp_player)
        (bind _returnvalue (and _array_element (== _array_index (`self.KeyValue`))))
        (if _returnvalue
          (`self.OpenDoor`)
          (break)))
      (if (not _returnvalue)
        (`|ExecutionSequence`
          (:`then_0`
            (`/Engine/EditorBlueprintResources/StandardMacros.DoOnce` false :!label _label_2
              (:`Completed`
                (bind _returnvalue_2 (`|CreateWidget` "/Game/JacobStuff/W_KeyDoor.W_KeyDoor_C"))
                (`UserWidget.AddToViewport` _returnvalue_2 0)
                (`KismetSystemLibrary.Delay` 4.0)
                (`Widget.RemoveFromParent` _returnvalue_2)
                (goto _label_2 :!via `Reset`))))
          (:`then_1`
            (goto _label :!via `Reset`)))))))

(fn `UserConstructionScript`)