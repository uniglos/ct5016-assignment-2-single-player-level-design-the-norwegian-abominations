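; BP_DoorKey is a key pickup that registers a door key on the player when its box is overlapped.
; Any overlap plays a pickup sound; if the actor is BP_Player, it inserts true into the player's Key array at index KeyValue.
; It then shows the W_KeyPickup widget and destroys its collision box and meshes.
; After a short delay, it removes the widget and destroys itself.
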(event `self.Box.OnComponentBeginOverlap`
  (params (OverlappedComponent :type "PrimitiveComponent Object Reference") (OtherActor :type "Actor Object Reference") (OtherComp :type "PrimitiveComponent Object Reference") (OtherBodyIndex :type Integer) (bFromSweep :type Boolean) (SweepResult :type "HitResult Structure (by ref)"))
  (`GameplayStatics.PlaySoundAtLocation` "/Game/PrototypeWeap/Sound/Pistol/Pistol_AmmoPickup.Pistol_AmmoPickup" (`self.K2_GetActorLocation`) (struct) 1.0 1.0 0.0 null null null null)
  (bind _asbp_player (cast `/Game/Blueprints/BP_Player` OtherActor))
  (`KismetArrayLibrary.Array_Insert` (`/Game/Blueprints/BP_Player.Key` _asbp_player) true (`self.KeyValue`))
  (bind _returnvalue (`|CreateWidget` "/Game/JacobStuff/W_KeyPickup.W_KeyPickup_C"))
  (`UserWidget.AddToViewport` _returnvalue 0)
  (`ActorComponent.K2_DestroyComponent` (`self.Box`))
  (`ActorComponent.K2_DestroyComponent` (`self.StaticMesh`))
  (`ActorComponent.K2_DestroyComponent` (`self.StaticMesh1`))
  (`ActorComponent.K2_DestroyComponent` (`self.StaticMesh2`))
  (`KismetSystemLibrary.Delay` 3.0)
  (`Widget.RemoveFromParent` _returnvalue)
  (`self.K2_DestroyActor`))

(fn `UserConstructionScript`)