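; BP_Lift is an elevator that carries its Floor component between a raised position and a lowered one.
; When an actor tagged Player enters BoxTrigger, it waits briefly, then plays the LiftDOWN or LiftUP timeline according to CanGoDown.
; Each timeline lerps the floor's relative location without sweep.
; CanGoDown flips after a delay started from the timeline's Update pin rather than Finished.
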(event `self.BoxTrigger.OnComponentBeginOverlap`
  (params (OverlappedComponent :type "PrimitiveComponent Object Reference") (OtherActor :type "Actor Object Reference") (OtherComp :type "PrimitiveComponent Object Reference") (OtherBodyIndex :type Integer) (bFromSweep :type Boolean) (SweepResult :type "HitResult Structure (by ref)"))
  (if (`self.ActorHasTag` OtherActor "Player")
    (if (`self.CanGoDown?`)
      (`KismetSystemLibrary.Delay` 2.0)
      (bind (_direction _movement) (`Timeline|LiftDOWN`)
        (:`Update`
          (`SceneComponent.K2_SetRelativeLocation` (`self.Floor`) (`KismetMathLibrary.VLerp` (0.0 0.0 0.0) (0.0 0.0 -345.0) _movement) false false)
          (`KismetSystemLibrary.Delay` 5.0)
          (set `self.CanGoDown?` false)))
      (else
        (`KismetSystemLibrary.Delay` 2.0)
        (bind (_direction_2 _movement_2) (`Timeline|LiftUP`)
          (:`Update`
            (`SceneComponent.K2_SetRelativeLocation` (`self.Floor`) (`KismetMathLibrary.VLerp` (0.0 0.0 -345.0) (0.0 0.0 0.0) _movement_2) false false)
            (`KismetSystemLibrary.Delay` 5.0)
            (set `self.CanGoDown?` true)))))))

(fn `UserConstructionScript`)