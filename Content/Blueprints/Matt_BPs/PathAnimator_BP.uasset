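; PathAnimator_BP moves an array of actors along a spline while BP_Player overlaps its trigger.
; Tick checks the trigger and plays a timeline whose rate derives from TimelineLength; its alpha maps to distance along the spline.
; Each actor is offset by its array index times OffsetBetweenActors, wrapping once past the spline end, and only location is set.
; The construction script pre-places the actors at those offsets.
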(event `self.ReceiveBeginPlay`
  (`TimelineComponent.SetPlayRate` (`self.Timeline`) (/ 1.0 (`self.Timeline Length`))))

(event `self.ReceiveTick`
  (params (DeltaSeconds :type "Float (single-precision)"))
  (if (`KismetArrayLibrary.Array_IsNotEmpty` (`self.GetOverlappingActors` (`self.Trigger`) "/Game/Blueprints/BP_Player.BP_Player_C"))
    (`self.Play Timeline`)))

(event `Play Timeline`
  (bind _returnvalue (`SplineComponent.GetSplineLength` (`self.Spline`)))
  (bind (_direction _alpha) (`Timeline|Timeline`)
    (:`Update`
      (for (_array_element _array_index) (`self.Actor`)
        (bind _output_get (set `self.Distance Along Spline` (+ (`KismetMathLibrary.Lerp` 0.0 (`SplineComponent.GetSplineLength` (`self.Spline`)) _alpha) (* _array_index (`self.Offset Between Actors`)))))
        (if (> _output_get _returnvalue)
          (set `self.Distance Along Spline` (- (`self.Distance Along Spline`) _returnvalue)))
        (`self.K2_SetActorLocation` _array_element (`SplineComponent.GetLocationAtDistanceAlongSpline` (`self.Spline`) (`self.Distance Along Spline`) "World") false false)))))

(fn `UserConstructionScript`
  (for (_array_element _array_index) (`self.Actor`)
    (`self.K2_SetActorLocation` _array_element (`SplineComponent.GetLocationAtDistanceAlongSpline` (`self.Spline`) (* (`self.Offset Between Actors`) _array_index) "World") false false)))